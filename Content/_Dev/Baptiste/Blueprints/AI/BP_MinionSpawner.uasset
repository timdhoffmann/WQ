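; BP_MinionSpawner is an actor that spawns a limited number of AI minions around a spawn zone.
; While tickets remain, Tick runs through a Delay that paces spawning by SpawnDelay, then spawns AIToSpawn with BT_Minion and decrements TicketCount.
; Spawn points are random within a box sized from the SpawnZone sphere's radius, and minions take the spawner's rotation.
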(event `self.ReceiveTick`
  (params (DeltaSeconds :type "Float (single-precision)"))
  (bind _spawnzone (`self.SpawnZone`))
  (if (> (`self.TicketCount`) 0)
    (`KismetSystemLibrary.Delay` (`self.SpawnDelay`))
    (`AIBlueprintHelperLibrary.SpawnAIFromClass` (`self.AIToSpawn`) "/Game/_Dev/Baptiste/AI/BT_Minion.BT_Minion" (`KismetMathLibrary.RandomPointInBoundingBox` (`SceneComponent.K2_GetComponentLocation` _spawnzone) (`KismetMathLibrary.Conv_DoubleToVector` (`SphereComponent.GetScaledSphereRadius` _spawnzone))) (`self.K2_GetActorRotation`))
    (bind _result (`/Engine/EditorBlueprintResources/StandardMacros.DecrementInt` (`self.TicketCount`))
      (:`  `
        (set `self.TicketCount` _result)))))

(fn `UserConstructionScript`)