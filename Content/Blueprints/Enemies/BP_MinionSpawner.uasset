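; Minion spawner actor that spawns AI enemies at random reachable points within its SpawnZone sphere.
; Each Tick it asks the game instance's SpawnDirector whether the harasser count is below this spawner's cap and the spawner is suitable.
; After a delay, it increments that shared count, spawns the configured pawn with its behavior tree and records itself as the minion's SpawnOrigin.
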(event `self.ReceiveTick`
  (params (DeltaSeconds :type "Float (single-precision)"))
  (bind _spawnzone (`self.SpawnZone`))
  (bind _aswqgame_instance (cast `WQGameInstance` (`GameplayStatics.GetGameInstance`)))
  (bind _returnvalue (`WQGameInstance.SpawnDirector` _aswqgame_instance))
  (bind _numberharasser (`SpawnDirector.NumberHarasser` _returnvalue))
  (if (not (>= _numberharasser (`self.MaxNumberHarasserOnMap`)))
    (bind _returnvalue_2 (`SpawnDirector.IsSpawnerSuitable` _returnvalue null))
    (if _returnvalue_2
      (`KismetSystemLibrary.Delay` (`self.SpawnDelay`))
      (set `SpawnDirector.NumberHarasser` (+ _numberharasser 1) _returnvalue)
      (bind _returnvalue_3 (`AIBlueprintHelperLibrary.SpawnAIFromClass` (`self.AIToSpawn`) (`self.AIBehavior`) (`NavigationSystemV1.K2_GetRandomReachablePointInRadius` (`SceneComponent.K2_GetComponentLocation` _spawnzone) (`SphereComponent.GetScaledSphereRadius` _spawnzone) null null) (`self.K2_GetActorRotation`)))
      (bind _aswqaicharacter (cast `WQAICharacter` _returnvalue_3))
      (set `WQAICharacter.SpawnOrigin` self _aswqaicharacter))))

(fn `UserConstructionScript`)